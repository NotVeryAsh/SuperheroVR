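; BP_Building_V3_Corner_Basement is a modular city building prefab for a corner basement piece with configurable materials.
; Its construction script applies Brick, Concrete, Wood, Metal and Glass material variables to slots on StaticMesh2, and a Cover material to StaticMesh.
; The event graph holds only disabled default events, so the actor has no runtime logic.
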(event EventBeginPlay)

(event Collision|EventActorBeginOverlap
  (params (OtherActor :type Actor%20Object%20Reference)))

(event EventTick
  (params (DeltaSeconds :type Float%20%28single-precision%29)))

(fn ConstructionScript
  (Rendering|Material|SetMaterial (Variables|Default|GetStaticMesh2) 5 (Variables|Default|GetBrick))
  (Rendering|Material|SetMaterial (Variables|Default|GetStaticMesh2) 1 (Variables|Default|GetConcrete))
  (Rendering|Material|SetMaterial (Variables|Default|GetStaticMesh2) 2 (Variables|Default|GetWood))
  (Rendering|Material|SetMaterial (Variables|Default|GetStaticMesh2) 0 (Variables|Default|GetMetal))
  (Rendering|Material|SetMaterial (Variables|Default|GetStaticMesh) 0 (Variables|Default|GetCover))
  (Rendering|Material|SetMaterial (Variables|Default|GetStaticMesh2) 3 (Variables|Default|GetGlass)))