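; BP_Shop_V2 is a shop building prefab in the CRCityPack city asset pack.
; Its construction script assigns brick, concrete, wood and glass materials to selected slots of the SMBApartmentDoorV1 mesh component.
; BeginPlay is empty, so the Blueprint adds no runtime behavior.
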(event EventBeginPlay)

(fn ConstructionScript
  (bind _sm_b_apartment_door_v1 (Variables|Default|GetSM_B_Apartment_Door_V1))
  (bind _concrete (Variables|Default|GetConcrete))
  (bind _glass (Variables|Default|GetGlass))
  (bind _sm_b_apartment_door_v1_2 (Variables|Default|GetSM_B_Apartment_Door_V1))
  (bind _sm_b_apartment_door_v1_3 (Variables|Default|GetSM_B_Apartment_Door_V1))
  (Rendering|Material|SetMaterial _sm_b_apartment_door_v1_3 3 (Variables|Default|GetBrick))
  (Rendering|Material|SetMaterial _sm_b_apartment_door_v1_3 0 _concrete)
  (Rendering|Material|SetMaterial _sm_b_apartment_door_v1_2 2 _concrete)
  (Rendering|Material|SetMaterial _sm_b_apartment_door_v1_2 4 (Variables|Default|GetWood))
  (Rendering|Material|SetMaterial _sm_b_apartment_door_v1 5 _glass)
  (Rendering|Material|SetMaterial _sm_b_apartment_door_v1 6 _glass))