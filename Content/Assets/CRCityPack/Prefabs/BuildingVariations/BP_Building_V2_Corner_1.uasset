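; BP_Building_V2_Corner_1 is a corner building variation prefab from the CRCityPack city asset pack.
; Its construction script applies brick, concrete, wood and glass materials to specific slots of the SMBApartmentDoorV1 component, with brick covering two slots.
; The event graph holds only disabled default events, so the Blueprint adds no runtime logic.
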(event EventBeginPlay)

(event Collision|EventActorBeginOverlap
  (params (OtherActor :type Actor%20Object%20Reference)))

(event EventTick
  (params (DeltaSeconds :type Float%20%28single-precision%29)))

(fn ConstructionScript
  (bind _sm_b_apartment_door_v1 (Variables|Default|GetSM_B_Apartment_Door_V1))
  (bind _brick (Variables|Default|GetBrick))
  (Rendering|Material|SetMaterial _sm_b_apartment_door_v1 2 _brick)
  (Rendering|Material|SetMaterial _sm_b_apartment_door_v1 7 _brick)
  (Rendering|Material|SetMaterial (Variables|Default|GetSM_B_Apartment_Door_V1) 1 (Variables|Default|GetConcrete))
  (Rendering|Material|SetMaterial (Variables|Default|GetSM_B_Apartment_Door_V1) 3 (Variables|Default|GetWood))
  (Rendering|Material|SetMaterial (Variables|Default|GetSM_B_Apartment_Door_V1) 4 (Variables|Default|GetGlass)))