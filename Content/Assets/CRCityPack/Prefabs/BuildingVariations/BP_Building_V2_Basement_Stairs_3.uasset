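; BP_Building_V2_Basement_Stairs_3 is a city pack building prefab, named as a basement stairs variation.
; Its construction script applies Brick, Concrete, Wood, Metal and Glass materials to fixed slots on the StaticMesh5 component, leaving slot 4 untouched.
; The event graph holds only disabled stub events, so it adds no runtime logic.
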(event EventBeginPlay)

(event Collision|EventActorBeginOverlap
  (params (OtherActor :type Actor%20Object%20Reference)))

(event EventTick
  (params (DeltaSeconds :type Float%20%28single-precision%29)))

(fn ConstructionScript
  (bind _staticmesh5 (Variables|Default|GetStaticMesh5))
  (Rendering|Material|SetMaterial (Variables|Default|GetStaticMesh5) 1 (Variables|Default|GetBrick))
  (Rendering|Material|SetMaterial (Variables|Default|GetStaticMesh5) 0 (Variables|Default|GetConcrete))
  (Rendering|Material|SetMaterial _staticmesh5 2 (Variables|Default|GetWood))
  (Rendering|Material|SetMaterial _staticmesh5 5 (Variables|Default|GetMetal))
  (Rendering|Material|SetMaterial (Variables|Default|GetStaticMesh5) 3 (Variables|Default|GetGlass)))