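; BP_Building_V2_Basement_1 is a city-pack building prefab for a basement variation, with no gameplay logic.
; Its construction script assigns Brick, Concrete, Wood, Metal and Glass material variables to specific slots on StaticMesh2, with Concrete covering several slots.
; The event graph holds only disabled placeholder events.
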(event EventBeginPlay)

(event Collision|EventActorBeginOverlap
  (params (OtherActor :type Actor%20Object%20Reference)))

(event EventTick
  (params (DeltaSeconds :type Float%20%28single-precision%29)))

(fn ConstructionScript
  (bind _staticmesh2 (Variables|Default|GetStaticMesh2))
  (bind _concrete (Variables|Default|GetConcrete))
  (Rendering|Material|SetMaterial (Variables|Default|GetStaticMesh2) 4 (Variables|Default|GetBrick))
  (Rendering|Material|SetMaterial _staticmesh2 1 _concrete)
  (Rendering|Material|SetMaterial _staticmesh2 8 _concrete)
  (Rendering|Material|SetMaterial _staticmesh2 9 _concrete)
  (Rendering|Material|SetMaterial (Variables|Default|GetStaticMesh2) 2 (Variables|Default|GetWood))
  (Rendering|Material|SetMaterial (Variables|Default|GetStaticMesh2) 5 (Variables|Default|GetMetal))
  (Rendering|Material|SetMaterial (Variables|Default|GetStaticMesh2) 3 (Variables|Default|GetGlass)))