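; BP_Building_V4 is a building prefab actor from the CRCityPack city asset pack.
; Its construction script applies the Brick, Concrete, Wood and Glass materials to separate material slots on the SMBApartmentDoorV1 component.
; The event graph holds only disabled placeholder events, so the actor has no gameplay logic.
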(event EventBeginPlay)

(event Collision|EventActorBeginOverlap
  (params (OtherActor :type Actor%20Object%20Reference)))

(event EventTick
  (params (DeltaSeconds :type Float%20%28single-precision%29)))

(fn ConstructionScript
  (Rendering|Material|SetMaterial (Variables|Default|GetSM_B_Apartment_Door_V1) 2 (Variables|Default|GetBrick))
  (Rendering|Material|SetMaterial (Variables|Default|GetSM_B_Apartment_Door_V1) 1 (Variables|Default|GetConcrete))
  (Rendering|Material|SetMaterial (Variables|Default|GetSM_B_Apartment_Door_V1) 3 (Variables|Default|GetWood))
  (Rendering|Material|SetMaterial (Variables|Default|GetSM_B_Apartment_Door_V1) 4 (Variables|Default|GetGlass)))