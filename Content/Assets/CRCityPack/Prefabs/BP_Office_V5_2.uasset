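; Prefab office building (V5_2 variant) from the CRCityPack, assembled from static mesh components including a bottom section.
; The construction script applies the Concrete material to slot 0 of all twelve referenced meshes and Glass to slot 1 of all but StaticMesh10, so the building's look is driven from two materials.
; The event graph holds only disabled stub events, so it has no runtime logic.
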(event EventBeginPlay)

(event Collision|EventActorBeginOverlap
  (params (OtherActor :type Actor%20Object%20Reference)))

(event EventTick
  (params (DeltaSeconds :type Float%20%28single-precision%29)))

(fn ConstructionScript
  (Rendering|Material|SetMaterial (Variables|Default|GetStaticMesh4) 0 (Variables|Default|GetConcrete))
  (Rendering|Material|SetMaterial (Variables|Default|GetStaticMesh2) 1 (Variables|Default|GetGlass)))