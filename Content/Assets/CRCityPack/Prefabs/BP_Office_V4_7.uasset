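; BP_Office_V4_7 is a modular office building prefab from the CR City Pack, assembled from static mesh components.
; Its construction script applies Brick, Concrete, Glass and Cover material variables to the window, door and cover meshes so the building's look can be set in one place.
; The door uses a different slot order for concrete and glass than the window pieces, and the event graph is empty.
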(event EventBeginPlay)

(event Collision|EventActorBeginOverlap
  (params (OtherActor :type Actor%20Object%20Reference)))

(event EventTick
  (params (DeltaSeconds :type Float%20%28single-precision%29)))

(fn ConstructionScript
  (bind _concrete (Variables|Default|GetConcrete))
  (bind _glass (Variables|Default|GetGlass))
  (Rendering|Material|SetMaterial (Variables|Default|GetSM_B_OfficeBlock_V3_Window_1) 0 (Variables|Default|GetBrick))
  (Rendering|Material|SetMaterial (Variables|Default|GetSM_B_OfficeBlock_V3_Window_1) 2 _concrete)
  (Rendering|Material|SetMaterial (Variables|Default|GetSM_B_OfficeBlock_V3_Door) 1 _concrete)
  (Rendering|Material|SetMaterial (Variables|Default|GetStaticMesh26) 0 (Variables|Default|GetCover))
  (Rendering|Material|SetMaterial (Variables|Default|GetStaticMesh3) 1 _glass)
  (Rendering|Material|SetMaterial (Variables|Default|GetSM_B_OfficeBlock_V3_Door) 2 _glass))