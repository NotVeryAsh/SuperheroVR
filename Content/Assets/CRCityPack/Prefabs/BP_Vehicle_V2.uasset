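; BP_Vehicle_V2 is a muscle car prop that drives along a referenced track's spline when ActiveVehicle is set.
; A timeline scaled by Duration and started at VehicleStartOffset maps its alpha to spline distance, setting the actor's location and rotation.
; Left and right wheel timelines spin the wheel meshes on roll at WheelSpeed.
; The construction script applies the body material and toggles three spotlights through EnableLights.
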(event Custom|MoveVehicle
  (bind _trackref (Variables|Default|GetTrackRef))
  (bind _splinepath (Variables|/Game/Assets/CRCityPack/Prefabs/BP_VehicleSpline.BP_VehicleSpline_C|GetSplinePath _trackref))
  (Components|Timeline|SetPlayRate (Variables|Default|GetVehicleMover) (/ 1.0 (Variables|Default|GetDuration)))
  (Components|Timeline|SetNewTime (Variables|Default|GetVehicleMover) (Variables|Default|GetVehicleStartOffset))
  (bind _alpha (Timeline|VehicleMover Play)
    (:Update
      (Variables|Default|SetAlpha _alpha)
      (Transformation|SetActorLocationAndRotation (Spline|GetLocationatDistanceAlongSpline _splinepath (Math|Float|Lerp 0.0 (Spline|GetSplineLength _splinepath) (Variables|Default|GetAlpha)) "World") (Spline|GetRotationatDistanceAlongSpline _splinepath (Math|Float|Lerp 0.0 (Spline|GetSplineLength _splinepath) (Variables|Default|GetAlpha)) "World")))))

(event EventBeginPlay
  (bind _staticmesh (Variables|Default|GetStaticMesh))
  (bind _sm_vehicle_muscle_v1_wheel (Variables|Default|GetSM_Vehicle_Muscle_V1_Wheel))
  (bind _staticmesh1 (Variables|Default|GetStaticMesh1))
  (bind _staticmesh2 (Variables|Default|GetStaticMesh2))
  (bind _relativerotation (Variables|/Script/Engine.SceneComponent|GetRelativeRotation _staticmesh1))
  (bind _relativerotation_2 (Variables|/Script/Engine.SceneComponent|GetRelativeRotation _staticmesh2))
  (bind _relativerotation_3 (Variables|/Script/Engine.SceneComponent|GetRelativeRotation _staticmesh))
  (bind _relativerotation_4 (Variables|/Script/Engine.SceneComponent|GetRelativeRotation _sm_vehicle_muscle_v1_wheel))
  (if (Variables|Default|GetActiveVehicle)
    (CallFunction|MoveVehicle)
    (Components|Timeline|SetPlayRate (Variables|Default|GetWheelL) (Variables|Default|GetWheelSpeed))
    (Utilities|FlowControl|Sequence
      (:then_0
        (bind _rotate (Timeline|WheelR PlayFromStart)
          (:Update
            (Transformation|SetRelativeRotation _staticmesh (Math|Rotator|MakeRotator _rotate (.pitch _relativerotation_3) (.yaw _relativerotation_3)) false false)
            (Transformation|SetRelativeRotation _sm_vehicle_muscle_v1_wheel (Math|Rotator|MakeRotator _rotate (.pitch _relativerotation_4) (.yaw _relativerotation_4)) false false))))
      (:then_1
        (bind _rotate_2 (Timeline|WheelL PlayFromStart)
          (:Update
            (Transformation|SetRelativeRotation _staticmesh1 (Math|Rotator|MakeRotator _rotate_2 (.pitch _relativerotation) (.yaw _relativerotation)) false false)
            (Transformation|SetRelativeRotation _staticmesh2 (Math|Rotator|MakeRotator _rotate_2 (.pitch _relativerotation_2) (.yaw _relativerotation_2)) false false)))))))

(fn ConstructionScript
  (bind _spotlight1 (Variables|Default|GetSpotLight1))
  (Rendering|Material|SetMaterial (Variables|Default|GetSM_Vehicle_Muscle_V1_Body) 0 (Variables|Default|GetColor))
  (if (Variables|Default|GetEnableLights)
    (Rendering|SetVisibility _spotlight1 true false)
    (else
      (Rendering|SetVisibility _spotlight1 false false))))