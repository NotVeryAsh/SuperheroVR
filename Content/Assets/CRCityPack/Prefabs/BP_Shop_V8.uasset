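; BP_Shop_V8 is a modular shop building prefab from the CRCityPack city asset pack, assembled from static mesh components such as walls, windows and a door.
; Its construction script applies Brick, Concrete and two Glass material variables to specific material slots across groups of meshes, so each instance can be restyled.
; The event graph holds only disabled placeholder events, so it has no runtime logic, and the Covers variable is unused.
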(event EventBeginPlay)

(event Collision|EventActorBeginOverlap
  (params (OtherActor :type Actor%20Object%20Reference)))

(event EventTick
  (params (DeltaSeconds :type Float%20%28single-precision%29)))

(fn ConstructionScript
  (bind _concrete (Variables|Default|GetConcrete))
  (Rendering|Material|SetMaterial (Variables|Default|GetStaticMesh1) 0 (Variables|Default|GetBrick))
  (Rendering|Material|SetMaterial (Variables|Default|GetStaticMesh4) 19 0)
  (Rendering|Material|SetMaterial (Variables|Default|GetStaticMesh1) 1 _concrete)
  (Rendering|Material|SetMaterial (Variables|Default|GetSM_B_Apartment_Door_V1) 0 _concrete)
  (Rendering|Material|SetMaterial (Variables|Default|GetStaticMesh27) 3 (Variables|Default|GetGlass%201))
  (Rendering|Material|SetMaterial (Variables|Default|GetStaticMesh19) 3 (Variables|Default|GetGlass%202)))