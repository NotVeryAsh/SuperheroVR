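; Modular city building prefab, the basement piece of Building V5, assembled from apartment door, window, roof and other static mesh components.
; The construction script assigns Brick, Concrete, Wood and Glass materials to matching slots across the door, window and generic meshes.
; The roof receives only Concrete, and one extra mesh slot takes Metal.
; It has no runtime logic, as the event graph holds only disabled default events.
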(event EventBeginPlay)

(event Collision|EventActorBeginOverlap
  (params (OtherActor :type Actor%20Object%20Reference)))

(event EventTick
  (params (DeltaSeconds :type Float%20%28single-precision%29)))

(fn ConstructionScript
  (bind _concrete (Variables|Default|GetConcrete))
  (Rendering|Material|SetMaterial (Variables|Default|GetSM_B_Apartment_Door_V1) 0 (Variables|Default|GetBrick))
  (Rendering|Material|SetMaterial (Variables|Default|GetStaticMesh2) 1 _concrete)
  (Rendering|Material|SetMaterial (Variables|Default|GetSM_B_Apartment_Roof_V1) 0 _concrete)
  (Rendering|Material|SetMaterial (Variables|Default|GetSM_B_Apartment_Door_V1) 2 (Variables|Default|GetWood))
  (Rendering|Material|SetMaterial (Variables|Default|GetStaticMesh2) 4 (Variables|Default|GetMetal))
  (Rendering|Material|SetMaterial (Variables|Default|GetStaticMesh1) 3 (Variables|Default|GetGlass)))